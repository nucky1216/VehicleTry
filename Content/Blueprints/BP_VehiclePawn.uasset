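; Self-driving vehicle pawn that steers toward a Target actor every tick.
; GetSteer takes the flattened direction to Target, scales its clamped angle from the forward vector into a steer amount, and signs it by a dot product with the right vector.
; Tick feeds that steer to the vehicle movement component and sets throttle higher the straighter the wheel.
; Debug arrows and printed values expose heading, angle, steer, speed and throttle.
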(event `self.ReceiveTick`
  (params (DeltaSeconds :type "Float (single-precision)"))
  (bind _steer (`self.GetSteer`))
  (bind _vehiclemovementcomponent (`self.VehicleMovementComponent`))
  (bind _returnvalue (+ 0.6 (* (- 1.0 (`KismetMathLibrary.Abs` _steer)) 0.5)))
  (`ChaosVehicleMovementComponent.SetSteeringInput` _vehiclemovementcomponent _steer)
  (`ChaosVehicleMovementComponent.SetThrottleInput` _vehiclemovementcomponent _returnvalue)
  (`KismetSystemLibrary.PrintString` (`KismetStringLibrary.Conv_DoubleToString` _returnvalue)))

(fn `GetSteer`
  (returns (Steer :type "Float (double-precision)"))
  (bind _returnvalue (`self.K2_GetActorLocation`))
  (bind _returnvalue_2 (`self.K2_GetActorLocation`))
  (bind _returnvalue_3 (`KismetMathLibrary.Normal` (* (- (`self.K2_GetActorLocation` (`self.Target`)) (`self.K2_GetActorLocation`)) (1.0 1.0 0.0))))
  (bind _returnvalue_4 (`KismetMathLibrary.SignOfFloat` (`KismetMathLibrary.Dot_VectorVector` _returnvalue_3 (`self.GetActorRightVector`))))
  (bind _returnvalue_5 (`KismetMathLibrary.DegAcos` (`KismetMathLibrary.Dot_VectorVector` _returnvalue_3 (`self.GetActorForwardVector`))))
  (bind _returnvalue_6 (* (/ (`KismetMathLibrary.ClampAngle` _returnvalue_5 0.0 40.0) 40.0) _returnvalue_4))
  (`KismetSystemLibrary.DrawDebugArrow` _returnvalue_2 (+ _returnvalue_2 (* _returnvalue_3 800.0)) 30.0 (struct :`R` 0.25 :`A` 1.0) 0.035 15.0)
  (`KismetSystemLibrary.DrawDebugArrow` _returnvalue (+ (* (`self.GetActorForwardVector`) 800.0) _returnvalue) 30.0 (struct :`R` 0.012454 :`G` 0.084508 :`B` 0.25 :`A` 1.0) 0.035 15.0)
  (`KismetSystemLibrary.PrintString` (`KismetStringLibrary.Concat_StrStr` "Angle:" (`KismetStringLibrary.Conv_DoubleToString` _returnvalue_5) " Sign:" (`KismetStringLibrary.Conv_DoubleToString` _returnvalue_4) " Steer:" (`KismetStringLibrary.Conv_DoubleToString` _returnvalue_6) " Speed:" (`KismetStringLibrary.Conv_DoubleToString` (`ChaosVehicleMovementComponent.GetForwardSpeed` (`self.VehicleMovementComponent`)))))
  (return _returnvalue_6))

(fn `UserConstructionScript`)